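; BP_StartGamePlayerZone is a zone actor that starts the game once all players are ready, moving them to the game level.
; On BeginPlay it binds handlers to the start-timer dispatchers for started, ticked, canceled and completed.
; Each handler prints status or countdown text, and completion also performs a server travel to LVL_Game.
; The readiness and timer logic is not in this graph, which only reacts to those events.
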(event `onStartGameTimerStarted_Event`
  (`KismetSystemLibrary.PrintString` "All the players are ready, starting soon"))

(event `onStartGameTimerTicked_Event` :!signature `self.onStartGameTimerTicked`
  (params (remainingTimeBeforeStarting :type Integer))
  (`KismetSystemLibrary.PrintString` (`KismetStringLibrary.Concat_StrStr` "Game starting in : " (`KismetStringLibrary.Conv_IntToString` remainingTimeBeforeStarting) " seconds")))

(event `self.ReceiveBeginPlay`
  (`|ExecutionSequence`
    (:`then_0`
      (add `self.onStartGameTimerStarted` (delegate `onStartGameTimerStarted_Event`)))
    (:`then_1`
      (add `self.onStartGameTimerTicked` (delegate `onStartGameTimerTicked_Event`)))
    (:`then_2`
      (add `self.onStartGameTimerCanceled` (delegate `onStartGameTimerCanceled_Event`)))
    (:`then_3`
      (add `self.onStartGameCompleted` (delegate `onStartGameCompleted_Event_0`)))))

(event `onStartGameTimerCanceled_Event`
  (`KismetSystemLibrary.PrintString` "Game start canceled"))

(event `onStartGameCompleted_Event_0`
  (`KismetSystemLibrary.PrintString` "Game started")
  (`AdvancedSessionsLibrary.ServerTravel` "LVL_Game"))

(fn `UserConstructionScript`)