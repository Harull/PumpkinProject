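; BP_Player is the player Blueprint, whose only active logic sets up positional VOIP voice chat on BeginPlay.
; It adds a VOIP Talker, retries on a short delay until the PlayerState is valid, then registers the talker with it.
; It then sets the mic threshold and assigns voice settings that attach audio to the camera component with SA_VOIP attenuation.
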(event `self.ReceiveBeginPlay`
  (`self.InitializeVoiceChat`))

(event `InitializeVoiceChat`
  (bind _playerstate (`self.PlayerState`))
  ; https://www.youtube.com/watch?v=PVDzjOV2wUg
  (bind _returnvalue (`AddComponent|NODE_AddVOIPTalker-0`))
  (set `self.VOIPRef` _returnvalue)
  (`/Engine/EditorBlueprintResources/StandardMacros.IsValid` _playerstate :!label _label
    (:`Is Valid`
      (`VOIPTalker.RegisterWithPlayerState` (`self.VOIPRef`) _playerstate)
      (`VOIPStatics.SetMicThreshold` -1.0)
      (set `VOIPTalker.Settings` (make `VoiceSettings` (`self.GetComponentByClass` "/Script/Engine.CameraComponent") "/Game/GPP/VoiceChatRelated/SA_VOIP.SA_VOIP") (`self.VOIPRef`)))
    (:`Is Not Valid`
      (`KismetSystemLibrary.Delay` 0.2)
      (goto _label))))

(fn `UserConstructionScript`)