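; Custom PCG node "Generate Dynamic Flat Roof" that builds a flat roof mesh from input point data.
; Point locations, relative to ActorLocation, form a polygon that Geometry Script triangulates and simplifies to planar.
; The faces are offset by the negated RoofOffset, then the polygroup 1 triangles are deleted and UVs are scaled.
; The result leaves on the FlatRoof pin as PCG dynamic mesh data with the assigned material.
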(fn ExecutewithContext
  (params (InContext :type PCG%20Context%20Structure%20%28by%20ref%29) (Input :type PCG%20Data%20Collection%20Structure%20%28by%20ref%29))
  (Utilities|FlowControl|Sequence
    (:then_0
      (bind _result (Utilities|Set|ToArray (PCG|Input&Output|CustomInputLabels self)))
      (bind _returnvalue (Data|GetInputsbyPinLabel Input (Utilities|Array|Get(acopy) _result)))
      (if (Utilities|Array|IsEmpty _returnvalue)
        (return "")
        (else
          (bind _aspcgpoint_data (Utilities|Casting|CastToPCGPointData (.Data (PCG|TaggedData|BreakTaggedData (Utilities|Array|Get(acopy) _returnvalue))))
            (:then
              (LocalVariables|SetPoints%201 _aspcgpoint_data))
            (:CastFailed
              (return ""))))))
    (:then_1
      (PCG|FlowControl|PointLoop InContext (LocalVariables|GetPoints%201) 0)
      (bind _returnvalue_2 (Class|GeometryScriptLibraryMeshPoolFunctions|GetGlobalMeshPool))
      (bind _mesh (Utilities|RequestandReleaseComputeMesh _returnvalue_2)
        (:With%20Mesh
          (bind _output_get (LocalVariables|SetCreatedMesh _mesh))
          (bind _returnvalue_3 (Class|GeometryScriptLibraryMeshPrimitiveFunctions|AppendTriangulatedPolygon3D :TargetMesh _output_get :PrimitiveOptions (Utilities|Struct|MakeGeometryScriptPrimitiveOptions "SingleGroup" false "Uniform" 0) :PolygonVertices3D (Variables|Default|GetFlatRoofPosition) :Debug 0))
          (bind _returnvalue_4 (Class|GeometryScriptLibraryMeshSimplifyFunctions|ApplySimplifytoPlanar _returnvalue_3 (Utilities|Struct|MakeGeometryScriptPlanarSimplifyOptions 2.0 true) 0))
          (bind _returnvalue_5 (Class|GeometryScriptLibraryMeshModelingFunctions|ApplyMeshInsetOutsetFaces :TargetMesh _returnvalue_4 :Options (Utilities|Struct|MakeGeometryScriptMeshInsetOutsetFacesOptions (* (Variables|Default|GetRoofOffset) -1.0) true false 0.0 1.0 "EntireSelection" (Utilities|Struct|MakeGeometryScriptMeshEditPolygroupOptions "PreserveExisting" 1) 1.0) :Debug 0))
          (bind (_selection _returnvalue_6) (Class|GeometryScriptLibraryMeshSelectionFunctions|SelectMeshElementsbyPolygroup :TargetMesh _returnvalue_5 :PolygroupID 1))
          (bind _returnvalue_7 (Class|GeometryScriptLibraryMeshBasicEditFunctions|DeleteSelectedTrianglesfromMesh _returnvalue_6 _selection false))
          (GeometryScript|UVs|ScaleMeshUVs :TargetMesh _returnvalue_7 :Scale (Variables|Default|GetScaleUV) :Debug 0)
          (bind _returnvalue_8 (Game|ConstructObjectfromClass "/Script/PCGGeometryScriptInterop.PCGDynamicMeshData"))
          (bind _output_get_2 (LocalVariables|SetPCGDynamicMesh%201 _returnvalue_8))
          (Class|PCGDynamicMeshData|Initialize _output_get_2 (LocalVariables|GetCreatedMesh) (Utilities|Array|MakeArray (Variables|Default|GetMaterial)) false)
          (Class|GeometryScriptLibraryMeshPoolFunctions|DiscardGlobalMeshPool)
          (return (Utilities|Struct|MakePCGDataCollection (Utilities|Array|MakeArray (PCG|TaggedData|MakeTaggedData (LocalVariables|GetPCGDynamicMesh%201) 0 "FlatRoof")))))))))

(fn PointLoopBody
  (params (InContext :type PCG%20Context%20Structure%20%28by%20ref%29) (InData :type PCG%20Point%20Data%20Object%20Reference) (InPoint :type PCG%20Point%20Structure%20%28by%20ref%29) (OutMetadata :type PCG%20Metadata%20Object%20Reference) (Iteration :type Integer64))
  (Utilities|Array|Add (Variables|Default|GetFlatRoofPosition) (- (.location (Utilities|Struct|BreakPCGPoint InPoint)) (Variables|Default|GetActorLocation)))
  (return "" false))

(fn NodeTitleOverride
  (return "Generate Dynamic Flat Roof"))