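; BP_PumpkinChara is a player character Blueprint that sets up Enhanced Input and captures movement input.
; On possession by a player controller on the autonomous proxy, it adds the IMC_MouseLook mapping context and prints a debug string.
; IA_Move updates RightVelocityRatio and ForwardVelocityRatio from the normalized 2D input, on both trigger and completion.
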(event `self.ReceivePossessed`
  (params (NewController :type "Controller Object Reference"))
  (switch `ENetRole` (`self.GetLocalRole`)
    (:`ROLE_AutonomousProxy`
      (if (`Controller.IsPlayerController` NewController)
        (bind _asplayer_controller (cast `PlayerController` NewController))
        (`EnhancedInputSubsystemInterface.AddMappingContext` (pcsubsystem `EnhancedInputLocalPlayerSubsystem` _asplayer_controller) "/Game/Player/Input/IMC_MouseLook.IMC_MouseLook" 0 (struct))
        (`KismetSystemLibrary.PrintString` "Hello2")))))

(event `EnhancedInput|/Game/Player/Input/Actions/IA_Move`
  (params (ActionValue :type "Vector2D Structure") (ElapsedSeconds :type "Float (double-precision)") (TriggeredSeconds :type "Float (double-precision)") (InputAction :type "InputAction Object Reference" :default "/Game/Player/Input/Actions/IA_Move.IA_Move"))
  (bind (_returnvalue_x _returnvalue_y) (`KismetMathLibrary.BreakVector2D` (`KismetMathLibrary.Normal2D` ActionValue)))
  (:`Triggered`
    (`|ExecutionSequence` :!label _label
      (:`then_0`
        (set `self.RightVelocityRatio` _returnvalue_x))
      (:`then_1`
        (set `self.ForwardVelocityRatio` _returnvalue_y))))
  (:`Completed`
    (goto _label)))

(fn `UserConstructionScript`)